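; Actor component that tracks an integer health value for its owner in the ShootingGuy game.
; Hurt, Heal, FullHeal and Kill all route through SetHealth, which clamps to zero and MaxHealth and broadcasts OnHealthChanged, alongside OnHurt and OnHeal dispatchers.
; On BeginPlay it binds to its own OnHealthChanged and fires OnDeath whenever health is at or below zero.
; SetMaxHealth changes the cap without re-clamping current health.
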(event Custom|OnHealthChanged%20Event
  (params (New%20Health :type Integer))
  ;[1 1 1] Handle Death
  (if (<= New%20Health 0)
    (Default|CallOnDeath)))

(event EventBeginPlay
  ;[1 1 1] Handle Death
  (EventDispatchers|BindEventtoOnHealthChanged (delegate Custom|OnHealthChanged%20Event)))

(fn Hurt
  (params (Damage :type Integer))
  (Setters|SetHealth (- (Variables|Default|GetHealth) Damage))
  (Default|CallOnHurt Damage))

(fn Heal
  (params (Healing :type Integer))
  (Setters|SetHealth (+ Healing (Variables|Default|GetHealth)))
  (Default|CallOnHeal Healing))

(fn SetHealth
  (params (New%20Health :type Integer))
  (bind _output_get (Variables|Default|SetHealth (Math|Integer|Clamp(Integer) New%20Health 0 (Variables|Default|GetMaxHealth))))
  (Default|CallOnHealthChanged _output_get))

(fn FullHeal
  (CallFunction|Heal (Variables|Default|GetMaxHealth)))

(fn Kill
  (CallFunction|Hurt (Variables|Default|GetMaxHealth)))

(fn GetHealth
  (return (Variables|Default|GetHealth)))

(fn GetMaxHealth
  (return (Variables|Default|GetMaxHealth)))

(fn SetMaxHealth
  (params (New%20Max%20Health :type Integer))
  (Variables|Default|SetMaxHealth New%20Max%20Health))