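; BP_Dummy is a dummy actor in ShootingGuy that gives visual feedback when it is hurt.
; The construction script creates a dynamic instance of M_Dummy on the skeletal mesh.
; When the health component fires OnHurt, it stamps the current game time into the material's TimeHit parameter.
; It also restarts a timeline that drives the mesh's relative scale from its Hit track.
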(event OnHurt(BPC_HealthComponent)
  (params (Damage :type Integer))
  (Rendering|Material|SetScalarParameterValue (Variables|Default|GetMaterialInstance) "TimeHit" (Utilities|Time|GetTimeSeconds) :!class /Script/Engine.MaterialInstanceDynamic)
  (bind _hit (Timeline|Timeline_0 PlayFromStart)
    (:Update
      (Transformation|SetRelativeScale3D (Variables|Default|GetSkeletalMesh) (Math|Conversions|ToVector(Float) _hit)))))

(event EventBeginPlay)

(event Collision|EventActorBeginOverlap
  (params (OtherActor :type Actor%20Object%20Reference)))

(fn ConstructionScript
  (bind _returnvalue (Rendering|Material|CreateDynamicMaterialInstance (Variables|Default|GetSkeletalMesh) 0 "/Game/ShootingGuy/Materials/M_Dummy.M_Dummy" "None" :!class /Script/Engine.PrimitiveComponent))
  (Variables|Default|SetMaterialInstance _returnvalue))