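; Player pawn for a mouse-aimed shooter that moves, turns toward the cursor and fires.
; Each tick it feeds horizontal and vertical input, scaled by Speed, into AddMovementInput and optionally rotates PlayerMesh.
; Aiming flattens the deprojected mouse ray direction to XY rather than tracing a cursor hit point.
; Left click calls ShootingComponent.Shoot from the Arrow's location along the mesh's forward vector.
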(event EventBeginPlay
  (Variables|/Script/Engine.PlayerController|SetbShowMouseCursor (Game|GetPlayerController 0) true))

(event Collision|EventActorBeginOverlap
  (params (OtherActor :type Actor%20Object%20Reference)))

(event EventTick
  (params (DeltaSeconds :type Float%20%28single-precision%29))
  (CallFunction|LookatMouse)
  (CallFunction|HandleMovement))

(event Input|MouseEvents|LeftMouseButton
  (params (Key :type Key%20Structure :default "None"))
  (:Pressed
    (Default|Shoot (Variables|Default|GetShooting%20Component) (Transformation|GetWorldLocation (Variables|Default|GetArrow)) (CallFunction|GetLookDirection))))

(fn ConstructionScript)

(fn LookatMouse
  (bind _returnvalue (Transformation|GetActorLocation))
  (bind _returnvalue_2 (Game|GetPlayerController 0))
  (bind _worlddirection (Game|Player|ConvertMouseLocationToWorldSpace _returnvalue_2))
  (bind _returnvalue_3 (Math|Vector|MakeVector (.x _returnvalue) (.y _returnvalue) 0.0))
  (if (Variables|Default|GetbLookAtMouse)
    (Transformation|SetWorldRotation (Variables|Default|GetPlayer%20Mesh) (Math|Rotator|FindLookatRotation _returnvalue_3 (+ _returnvalue_3 (Math|Vector|MakeVector (.x _worlddirection) (.y _worlddirection) 0.0))) false false)))

(fn GetLookDirection
  (return (Math|Vector|GetForwardVector (Variables|Default|GetPlayer%20Mesh))))

(fn HandleMovement
  (Pawn|Input|AddMovementInput (* (Math|Vector|MakeVector (Input|AxisValues|GetHorizontalMovement) (Input|AxisValues|GetVerticalMovement) 0.0) (Variables|Default|GetSpeed)) 1.0 false))